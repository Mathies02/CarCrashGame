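; BP_Car is a car that travels along a spline path while carrying the player with it.
; A timeline, with play rate derived from TimeToFinish, drives the car's location and rotation along PathToFollow's spline by distance.
; Every Tick teleports the player character to the car's Arrow component, and BeginPlay starts the move and sets the car's rotation from that Arrow.
; The construction script applies CarMesh to the interior mesh.
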(event `self.ReceiveTick`
  (params (DeltaSeconds :type "Float (single-precision)"))
  (`self.K2_SetActorLocation` (`GameplayStatics.GetPlayerCharacter` 0) (`SceneComponent.K2_GetComponentLocation` (`self.Arrow`)) false true))

(event `self.ReceiveBeginPlay`
  (`self.Car_Move`)
  (`self.K2_SetActorRotation` (`SceneComponent.K2_GetComponentRotation` (`self.Arrow`)) true))

(event `Car_Move`
  (bind _path (`/Game/Car/BP_CarPath.Path` (`self.Path To Follow`)))
  (`TimelineComponent.SetPlayRate` (`self.Car_Movement`) (/ 1.0 (`self.Time To Finish`)))
  (bind (_direction _move_track) (`Timeline|Car_Movement`)
    (:`Update`
      (bind _returnvalue (`KismetMathLibrary.Lerp` 0.0 (`SplineComponent.GetSplineLength` _path) _move_track))
      (`self.K2_SetActorLocationAndRotation` (`SplineComponent.GetLocationAtDistanceAlongSpline` _path _returnvalue "World") (`SplineComponent.GetRotationAtDistanceAlongSpline` _path _returnvalue "World")))))

(fn `UserConstructionScript`
  (`StaticMeshComponent.SetStaticMesh` (`self.SM_CarInterior`) (`self.Car Mesh`)))