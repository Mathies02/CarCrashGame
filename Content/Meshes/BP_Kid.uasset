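; Kid with a balloon that walks a spline path and triggers the game's ending.
; Overlapping StartWalking plays the KidWalk timeline, scaled by TimeToWalk, moving both skeletal meshes along PathToWalk at fixed rotation.
; Overlapping Ending restores look input and shows the ending widget, then once only plays a scream and stops both animations.
; After a delay, it raises GameManager's LossCounter by an amount depending on HasWon and loads the main menu.
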(event `self.ReceiveBeginPlay`)

(event `self.Start Walking.OnComponentBeginOverlap`
  (params (OverlappedComponent :type "PrimitiveComponent Object Reference") (OtherActor :type "Actor Object Reference") (OtherComp :type "PrimitiveComponent Object Reference") (OtherBodyIndex :type Integer) (bFromSweep :type Boolean) (SweepResult :type "HitResult Structure (by ref)"))
  (bind _path_to_walk (`self.Path To Walk`))
  (`TimelineComponent.SetPlayRate` (`self.KidWalk`) (/ 1.0 (`self.Time To Walk`)))
  (bind (_direction _walk) (`Timeline|KidWalk`)
    (:`Update`
      (`SceneComponent.K2_SetWorldLocationAndRotation` (`self.SK_Kid`) (`SplineComponent.GetLocationAtDistanceAlongSpline` _path_to_walk (`KismetMathLibrary.Lerp` 0.0 (`SplineComponent.GetSplineLength` _path_to_walk) _walk) "World") (struct :`Yaw` 180.0) false false)
      (`SceneComponent.K2_SetWorldLocationAndRotation` (`self.SK_Balloon`) (`SplineComponent.GetLocationAtDistanceAlongSpline` _path_to_walk (`KismetMathLibrary.Lerp` 0.0 (`SplineComponent.GetSplineLength` _path_to_walk) _walk) "World") (struct :`Yaw` 180.0) false false))))

(event `self.Ending.OnComponentBeginOverlap`
  (params (OverlappedComponent :type "PrimitiveComponent Object Reference") (OtherActor :type "Actor Object Reference") (OtherComp :type "PrimitiveComponent Object Reference") (OtherBodyIndex :type Integer) (bFromSweep :type Boolean) (SweepResult :type "HitResult Structure (by ref)"))
  (`Controller.SetIgnoreLookInput` (`GameplayStatics.GetPlayerController` 0) false)
  (bind _returnvalue (`|CreateWidget` "/Game/UI/WB_Ending.WB_Ending_C"))
  (`UserWidget.AddToViewport` _returnvalue 0)
  (`/Engine/EditorBlueprintResources/StandardMacros.DoOnce` false
    (:`Completed`
      (`GameplayStatics.PlaySound2D` "/Game/Sound/Scream.Scream" 1.0 1.0 0.0 null null)
      (`SkeletalMeshComponent.SetEnableAnimation` (`self.SK_Kid`) false)
      (`SkeletalMeshComponent.SetEnableAnimation` (`self.SK_Balloon`) false)
      (`KismetSystemLibrary.Delay` 5.0)
      (bind _asgame_manager (cast `/Game/Blueprints/GameManager` (`GameplayStatics.GetGameInstance`)))
      (if (`/Game/Blueprints/GameManager.HasWon` _asgame_manager)
        (bind _losscounter (`/Game/Blueprints/GameManager.LossCounter` _asgame_manager))
        (set `/Game/Blueprints/GameManager.LossCounter` (+ _losscounter 100) _asgame_manager)
        (`GameplayStatics.OpenLevel` "MainMenuMap")
        (else
          (set `/Game/Blueprints/GameManager.LossCounter` (+ _losscounter 1) _asgame_manager)
          (`GameplayStatics.OpenLevel` "MainMenuMap"))))))

(fn `UserConstructionScript`)